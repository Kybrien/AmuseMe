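; AutoMoto is a simple drivable vehicle Blueprint steered through two input actions, AutoForward and AutoSides.
; AutoForward pushes the VoitureCommeTuVeux component along its forward vector with AddForce, scaled by the action value and Speed.
; AutoSides turns that component by setting its world rotation directly, combining it with a yaw step of action value times TurnSpeed, without delta-time scaling.
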(event `self.ReceiveBeginPlay`)

(event `EnhancedInput|/Game/2DAction/Input/AutoActions/AutoForward`
  (params (ActionValue :type "Float (double-precision)") (ElapsedSeconds :type "Float (double-precision)") (TriggeredSeconds :type "Float (double-precision)") (InputAction :type "InputAction Object Reference" :default "/Game/2DAction/Input/AutoActions/AutoForward.AutoForward"))
  (:`Triggered`
    (`PrimitiveComponent.AddForce` (`self.VoitureCommeTuVeux`) (* (* ActionValue (`self.Speed`)) (`SceneComponent.GetForwardVector` (`self.VoitureCommeTuVeux`))) "None" false)))

(event `EnhancedInput|/Game/2DAction/Input/AutoActions/AutoSides`
  (params (ActionValue :type "Float (double-precision)") (ElapsedSeconds :type "Float (double-precision)") (TriggeredSeconds :type "Float (double-precision)") (InputAction :type "InputAction Object Reference" :default "/Game/2DAction/Input/AutoActions/AutoSides.AutoSides"))
  (:`Triggered`
    (`SceneComponent.K2_SetWorldRotation` (`self.VoitureCommeTuVeux`) (`KismetMathLibrary.ComposeRotators` (`SceneComponent.K2_GetComponentRotation` (`self.VoitureCommeTuVeux`)) (`KismetMathLibrary.MakeRotator` 0.0 0.0 (* ActionValue (`self.TurnSpeed`)))) false false)))

(fn `UserConstructionScript`)