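; BP_ChambouleTOUT_Parent is the parent Blueprint for a physics-driven prop in the ChambouleTout (can knockdown) attraction, able to return to its starting place.
; BeginPlay caches the static mesh's world location.
; ResetPos switches physics off, teleports the mesh to that location, zeroes its world rotation instead of restoring the original, then turns physics back on.
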(event `self.ReceiveBeginPlay`
  ; Set Initial Location
  (set `self.initialPos` (`SceneComponent.K2_GetComponentLocation` (`self.StaticMesh`))))

(event `ResetPos`
  ; Reset Pos Function
  (`PrimitiveComponent.SetSimulatePhysics` (`self.StaticMesh`) false)
  (`SceneComponent.K2_SetWorldLocation` (`self.StaticMesh`) (`self.initialPos`) false true)
  (`SceneComponent.K2_SetWorldRotation` :`self` (`self.StaticMesh`))
  (`PrimitiveComponent.SetSimulatePhysics` (`self.StaticMesh`) true))

(fn `UserConstructionScript`)